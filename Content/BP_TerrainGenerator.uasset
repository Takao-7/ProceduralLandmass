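; Terrain generator actor that builds a map in the editor from its construction script, using a Configuration struct.
; When the ShouldGenerateMap check passes, it creates a PerlinNoiseGenerator if the configuration lacks a valid noise generator, then calls GenerateMap.
; It then clears the GenerateMap boolean, which makes that flag act as a one-shot trigger.
; The event graph holds no logic.
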(fn `UserConstructionScript`
  (bind (_configuration_numberofthreads _configuration_noisegenerator) (break `TerrainConfiguration` (`self.Configuration`)))
  (bind (_configuration_numberofthreads_2 _configuration_noisegenerator_2 _configuration_numvertices _configuration_mapscale _configuration_numchunks _configuration_amplitude _configuration_heightcurve _configuration_ditheringlodtransitions _configuration_lods) (break `TerrainConfiguration` (`self.Configuration`)))
  (`self.Should generate map`
    (:`Yes`
      (`/Engine/EditorBlueprintResources/StandardMacros.IsValid` (`KismetSystemLibrary.Conv_InterfaceToObject` _configuration_noisegenerator)
        (:`Is Valid`
          _)
        (:`Is Not Valid`
          (bind _returnvalue (`|GenericCreateObject` "/Script/ProceduralLandmass.PerlinNoiseGenerator" self))
          (set `self.Configuration` (make `TerrainConfiguration` _configuration_numberofthreads_2 _returnvalue _configuration_numvertices _configuration_mapscale _configuration_numchunks _configuration_amplitude _configuration_heightcurve _configuration_ditheringlodtransitions _configuration_lods))))
      (`self.GenerateMap`)
      (set `self.bGenerateMap` false))))